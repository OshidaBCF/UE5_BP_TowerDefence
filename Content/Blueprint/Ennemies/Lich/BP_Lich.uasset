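; BP_Lich is a Lich enemy that pursues the player for a short time, then dies on a timer.
; On BeginPlay it calls the parent logic and starts an AI MoveTo toward the first player pawn.
; The immediate output, independent of move success, starts a delay that then sets IsDead and detaches the controller pending destroy.
; Tick and overlap events are disabled.
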(event EventBeginPlay
  (|CallParentFunction)
  (AI|AIMoveTo self "0, 0, 0" (Game|Player|GetPlayerPawn 0) 5.0 false
    (:then
      (Utilities|FlowControl|Delay 6.0)
      (Variables|Default|SetIsDead true)
      (Class|Pawn|DetachfromControllerPendingDestroy))))

(event Collision|EventActorBeginOverlap
  (params (OtherActor :type Actor%20Object%20Reference))
  (|CallParentFunction OtherActor) ; This node is disabled and will not be called.\nDrag off pins to build functionality.
)

(event EventTick
  (params (DeltaSeconds :type Float%20%28single-precision%29))
  (|CallParentFunction DeltaSeconds) ; This node is disabled and will not be called.\nDrag off pins to build functionality.
)

(fn ConstructionScript
  (|CallParentFunction))