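; BP_Goblin is an enemy pawn that walks toward a randomly picked tower and can be killed by projectiles.
; On BeginPlay it picks among BP_Tower actors tagged "Alive" and issues an AI MoveTo to that location.
; A failed move flags it dead and detaches its controller.
; Capsule hits from first-person or standard projectiles destroy the projectile and decrement HP, clearing tags and destroying the goblin at zero.
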(event OnComponentHit(CapsuleComponent)
  (params (HitComponent :type Primitive%20Component%20Object%20Reference) (OtherActor :type Actor%20Object%20Reference) (OtherComp :type Primitive%20Component%20Object%20Reference) (NormalImpulse :type Vector :default "0, 0, 0") (Hit :type Hit%20Result%20Structure%20%28by%20ref%29))
  (bind _returnvalue (Utilities|GetClass OtherActor))
  (if (or (== _returnvalue "/Game/FirstPerson/Blueprints/BP_FirstPersonProjectile.BP_FirstPersonProjectile_C") (== _returnvalue "/Game/Blueprint/BP_Projectile.BP_Projectile_C"))
    (Actor|DestroyActor OtherActor)
    (bind _result (Math|Integer|DecrementInt (Variables|Default|GetHP))
      (:%20%20
        (if (<= _result 0)
          (Utilities|Array|Clear (Variables|Default|GetTags))
          (Actor|DestroyActor))))))

(event Custom|SelectTarget
  (bind _outactors (Actor|GetAllActorsOfClasswithTag "/Game/Blueprint/BP_Tower.BP_Tower_C" "Alive"))
  (AI|AIMoveTo self (Transformation|GetActorLocation (Utilities|Array|Get(acopy) _outactors (Math|Random|RandomInteger (- (Utilities|Array|Length _outactors) 1)))) 0 5.0 false
    (:then
      (Utilities|FlowControl|Delay 6.0))
    (:OnFail
      (Variables|Default|SetIsDead true)
      (Class|Pawn|DetachfromControllerPendingDestroy))))

(event EventBeginPlay
  (|CallParentFunction)
  (CallFunction|SelectTarget))

(event EventTick
  (params (DeltaSeconds :type Float%20%28single-precision%29))
  (|CallParentFunction DeltaSeconds) ; This node is disabled and will not be called.\nDrag off pins to build functionality.
)

(fn ConstructionScript
  (|CallParentFunction))