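; Hobgoblin enemy that walks toward a tower when it spawns.
; On BeginPlay it gathers BP_Tower actors tagged Alive and uses AIMoveTo toward a randomly indexed one, with an index range that leaves out the last tower.
; A closest-tower search and a death sequence that sets IsDead and detaches the controller are present but unconnected, so neither runs.
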(event EventBeginPlay
  (|CallParentFunction)
  (bind _outactors (Actor|GetAllActorsOfClasswithTag "/Game/Blueprint/BP_Tower.BP_Tower_C" "Alive"))
  (switch int (Utilities|Array|Length _outactors)
    (:Default
      (AI|AIMoveTo self (Transformation|GetActorLocation (Utilities|Array|Get(acopy) _outactors (Math|Random|RandomInteger (- (Utilities|Array|Length _outactors) 1)))) (Utilities|Array|Get(acopy) _outactors (Math|Random|RandomInteger (- (Utilities|Array|Length _outactors) 1))) 5.0 false
        (:then
          (Utilities|FlowControl|Delay 6.0))))))

(event Collision|EventActorBeginOverlap
  (params (OtherActor :type Actor%20Object%20Reference))
  (|CallParentFunction OtherActor) ; This node is disabled and will not be called.\nDrag off pins to build functionality.
)

(event EventTick
  (params (DeltaSeconds :type Float%20%28single-precision%29))
  (|CallParentFunction DeltaSeconds) ; This node is disabled and will not be called.\nDrag off pins to build functionality.
)

(fn ConstructionScript
  (|CallParentFunction))