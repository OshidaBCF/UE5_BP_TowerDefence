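; Homing Bullet Bill enemy projectile that chases the first player pawn and explodes on contact.
; Tick steers the static mesh toward the player at a set speed and shifts its smoke from grey to red as it closes in.
; Box hits, player overlaps or "Projectile"-tagged actors trigger the explosion and delayed destruction, also destroying that projectile.
; Player overlap calls KillPlayer, which is empty here.
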(event OnComponentHit(Box)
  (params (HitComponent :type Primitive%20Component%20Object%20Reference) (OtherActor :type Actor%20Object%20Reference) (OtherComp :type Primitive%20Component%20Object%20Reference) (NormalImpulse :type Vector :default "0, 0, 0") (Hit :type Hit%20Result%20Structure%20%28by%20ref%29))
  (bind _staticmesh (Variables|Default|GetStaticMesh))
  (Physics|SetSimulatePhysics _staticmesh false)
  (Collision|SetCollisionEnabled _staticmesh "NoCollision")
  (Rendering|SetVisibility _staticmesh false false)
  (Components|Activation|Activate (Variables|Default|GetExplosion) false)
  (Utilities|Array|Clear (Variables|Actor|GetTags))
  (Components|Activation|Deactivate (Variables|Default|GetSmoke))
  (Components|DestroyComponent (Variables|Default|GetBox))
  (Utilities|FlowControl|Delay 2.0)
  (Actor|DestroyActor))

(event OnComponentBeginOverlap(Box)
  (params (OverlappedComponent :type Primitive%20Component%20Object%20Reference) (OtherActor :type Actor%20Object%20Reference) (OtherComp :type Primitive%20Component%20Object%20Reference) (OtherBodyIndex :type Integer) (bFromSweep :type Boolean) (SweepResult :type Hit%20Result%20Structure%20%28by%20ref%29))
  (bind _staticmesh (Variables|Default|GetStaticMesh))
  (if (== OtherActor (Game|Player|GetPlayerPawn 0))
    (CallFunction|KillPlayer)
    (Physics|SetSimulatePhysics _staticmesh false :!label _label)
    (Collision|SetCollisionEnabled _staticmesh "NoCollision")
    (Rendering|SetVisibility _staticmesh false false)
    (Components|Activation|Activate (Variables|Default|GetExplosion) false)
    (Utilities|Array|Clear (Variables|Actor|GetTags))
    (Components|Activation|Deactivate (Variables|Default|GetSmoke))
    (Components|DestroyComponent (Variables|Default|GetBox))
    (Utilities|FlowControl|Delay 2.0)
    (Actor|DestroyActor)
    (elif (Actor|ActorHasTag OtherActor "Projectile")
      (Actor|DestroyActor OtherActor)
      (goto _label))))

(event EventBeginPlay)

(event Collision|EventActorBeginOverlap
  (params (OtherActor :type Actor%20Object%20Reference)))

(event EventTick
  (params (DeltaSeconds :type Float%20%28single-precision%29))
  (bind _returnvalue (Game|Player|GetPlayerPawn 0))
  (bind _staticmesh (Variables|Default|GetStaticMesh))
  (bind _returnvalue_2 (Transformation|GetWorldLocation _staticmesh))
  (bind _returnvalue_3 (Transformation|GetActorLocation _returnvalue))
  (bind _returnvalue_4 (- _returnvalue_3 _returnvalue_2))
  (bind _returnvalue_5 (Math|Vector|Normalize _returnvalue_4))
  (Transformation|SetWorldLocationAndRotation (Variables|Default|GetStaticMesh) (+ (* DeltaSeconds (Variables|Default|GetSpeed) _returnvalue_5) _returnvalue_2) (Math|Conversions|RotationFromXVector _returnvalue_5) false false)
  (Effects|Components|ParticleSystem|SetColorParameter (Variables|Default|GetSmoke) "Color" (Math|Color|Lerp(LinearColor) "(R=0.752942,G=0.070588,B=0.070588,A=1.000000)" "(R=0.752942,G=0.745404,B=0.737910,A=1.000000)" (Math|Float|MapRangeClamped (Math|Vector|VectorLength _returnvalue_4) 1.5e+02 6e+02 0.0 1.0))))

(fn ConstructionScript)

(fn KillPlayer
  (params (playerHit :type Actor%20Object%20Reference)))