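; BP_Plateform is a falling platform that drops after the player touches it and then resets.
; On BeginPlay it caches the static mesh's world location and rotation.
; When the player character hits the mesh, it waits briefly, enables physics simulation so the platform falls, then after another delay disables physics and restores the cached transform.
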(event OnComponentHit(StaticMesh)
  (params (HitComponent :type Primitive%20Component%20Object%20Reference) (OtherActor :type Actor%20Object%20Reference) (OtherComp :type Primitive%20Component%20Object%20Reference) (NormalImpulse :type Vector :default "0, 0, 0") (Hit :type Hit%20Result%20Structure%20%28by%20ref%29))
  (bind _staticmesh (Variables|Default|GetStaticMesh))
  (if (== OtherActor (Game|GetPlayerCharacter 0))
    (Utilities|FlowControl|Delay 2.0)
    (Physics|SetSimulatePhysics (Variables|Default|GetStaticMesh) true)
    (Utilities|FlowControl|Delay 3.0)
    (Physics|SetSimulatePhysics _staticmesh false)
    (Transformation|SetWorldLocationAndRotation _staticmesh (Variables|Default|GetDefaultLocation) (Variables|Default|GetDefaultRotation%20) false false)))

(event Collision|EventActorBeginOverlap
  (params (OtherActor :type Actor%20Object%20Reference)))

(event EventBeginPlay
  (bind _staticmesh (Variables|Default|GetStaticMesh))
  (Variables|Default|SetDefaultLocation (Transformation|GetWorldLocation _staticmesh))
  (Variables|Default|SetDefaultRotation%20 (Transformation|GetWorldRotation _staticmesh)))

(fn ConstructionScript)