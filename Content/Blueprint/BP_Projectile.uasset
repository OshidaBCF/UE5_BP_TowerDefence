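; Projectile actor built around a physics-driven Arrow component that destroys itself on a hit or after about twenty seconds.
; Hit notifications on the Arrow are switched off at spawn and enabled halfway through that lifetime.
; Each tick scales down the Arrow's vertical velocity in proportion to itself, frame time and a Gravity variable, damping vertical motion rather than adding constant downward acceleration.
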(event OnComponentHit(Arrow)
  (params (HitComponent :type Primitive%20Component%20Object%20Reference) (OtherActor :type Actor%20Object%20Reference) (OtherComp :type Primitive%20Component%20Object%20Reference) (NormalImpulse :type Vector :default "0, 0, 0") (Hit :type Hit%20Result%20Structure%20%28by%20ref%29))
  (Actor|DestroyActor))

(event EventBeginPlay
  (bind _arrow (Variables|Default|GetArrow))
  (Class|PrimitiveComponent|SetNotifyRigidBodyCollision _arrow false)
  (Utilities|FlowControl|Delay 1e+01)
  (Class|PrimitiveComponent|SetNotifyRigidBodyCollision _arrow true)
  (Utilities|FlowControl|Delay 1e+01)
  (Actor|DestroyActor))

(event Collision|EventActorBeginOverlap
  (params (OtherActor :type Actor%20Object%20Reference)))

(event EventTick
  (params (DeltaSeconds :type Float%20%28single-precision%29))
  (bind _arrow (Variables|Default|GetArrow))
  (bind _returnvalue (Physics|GetPhysicsLinearVelocity _arrow "None"))
  (Physics|SetPhysicsLinearVelocity _arrow (Math|Vector|MakeVector (.X (Math|Vector|BreakVector _returnvalue)) (.Y (Math|Vector|BreakVector _returnvalue)) (- (.Z (Math|Vector|BreakVector _returnvalue)) (* (.Z (Math|Vector|BreakVector _returnvalue)) (* DeltaSeconds (Variables|Default|Getgravity) 0.01)))) false "None"))

(fn ConstructionScript)