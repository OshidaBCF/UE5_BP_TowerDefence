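; BP_Shooting is a stationary-logic shooter actor that fires projectiles at the player when they are nearby.
; A looping timer started on BeginPlay triggers Shoot every two seconds, which checks that the player pawn is within range.
; It then spawns a BP_Projectile at its own location and launches it with an impulse on BulletSphere, aimed at the player's current position and scaled by ImpulseForce.
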(event Custom|Shoot
  (bind _returnvalue (Transformation|GetActorLocation))
  (if (<= (Transformation|GetDistanceTo (Game|Player|GetPlayerPawn 0)) 5e+02)
    (bind _returnvalue_2 (Game|SpawnActorfromClass "/Game/Blueprint/BP_Projectile.BP_Projectile_C" (Math|Conversions|ToTransform(Vector) _returnvalue) "Undefined" "MultiplyWithRoot" 0 0))
    (Physics|AddImpulse (Variables|/Game/Blueprint/BP_Projectile.BP_Projectile_C|GetBulletSphere _returnvalue_2) (* (Math|Vector|GetUnitDirection(Vector) _returnvalue (Transformation|GetActorLocation (Game|Player|GetPlayerPawn 0))) (Variables|Default|GetImpulseForce)) "None" false)))

(event EventBeginPlay
  (Utilities|Time|SetTimerbyEvent (delegate Custom|Shoot) 2.0 true))

(event Collision|EventActorBeginOverlap
  (params (OtherActor :type Actor%20Object%20Reference)))

(event EventTick
  (params (DeltaSeconds :type Float%20%28single-precision%29)))

(fn ConstructionScript)