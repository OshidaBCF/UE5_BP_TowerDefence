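; BP_FallingPlatform is a platform that drops after the player touches it and then resets.
; A hit on its static mesh by the player pawn starts a short delay, after which physics simulation is switched on so the mesh falls.
; After a further delay, physics is switched off and the mesh is moved back to the root component's world transform.
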(event OnComponentHit(StaticMesh)
  (params (HitComponent :type Primitive%20Component%20Object%20Reference) (OtherActor :type Actor%20Object%20Reference) (OtherComp :type Primitive%20Component%20Object%20Reference) (NormalImpulse :type Vector :default "0, 0, 0") (Hit :type Hit%20Result%20Structure%20%28by%20ref%29))
  (bind _staticmesh (Variables|Default|GetStaticMesh))
  (if (== OtherActor (Game|Player|GetPlayerPawn 0))
    (Utilities|FlowControl|Delay 2.0)
    (Physics|SetSimulatePhysics _staticmesh true)
    (Utilities|FlowControl|Delay 3.0)
    (Physics|SetSimulatePhysics _staticmesh false)
    (Transformation|SetWorldTransform _staticmesh (Transformation|GetWorldTransform (Variables|Default|GetDefaultSceneRoot)) false false)))

(event EventBeginPlay)

(event Collision|EventActorBeginOverlap
  (params (OtherActor :type Actor%20Object%20Reference)))

(event EventTick
  (params (DeltaSeconds :type Float%20%28single-precision%29)))

(fn ConstructionScript)