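; BP_VanishingClouds is a cloud object that fades out and loses collision after the player's pawn hits it, then returns.
; The construction script creates a dynamic material instance, whose Transparency parameter is driven by two timelines scaled to PhaseTime.
; After a delay the first timeline fades the mesh, collision switches off for RespawnTime, then collision returns and the second timeline plays in reverse.
; An AlreadyHit flag blocks retriggering until the cycle finishes.
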(event OnComponentHit(StaticMesh)
  (params (HitComponent :type Primitive%20Component%20Object%20Reference) (OtherActor :type Actor%20Object%20Reference) (OtherComp :type Primitive%20Component%20Object%20Reference) (NormalImpulse :type Vector :default "0, 0, 0") (Hit :type Hit%20Result%20Structure%20%28by%20ref%29))
  (bind _staticmesh (Variables|Default|GetStaticMesh))
  (bind _cloudpaint (Variables|Default|GetCloudPaint))
  (if (and (== OtherActor (Game|Player|GetPlayerPawn 0)) (not (Variables|Default|GetalreadyHit)))
    (Variables|Default|SetalreadyHit true)
    (Utilities|FlowControl|Delay (Variables|Default|GettimeBeforePhase))
    (Rendering|Material|SetMaterial (Variables|Default|GetStaticMesh) 0 _cloudpaint)
    (Components|Timeline|SetPlayRate (Variables|Default|GetTransparancy) (/ 2.0 (Variables|Default|GetphaseTime)))
    (bind _transparency (Timeline|Transparancy PlayFromStart)
      (:Update
        (Rendering|Material|SetScalarParameterValue _cloudpaint "Transparency" _transparency :!class /Script/Engine.MaterialInstanceDynamic))
      (:Finished
        (Collision|SetCollisionEnabled _staticmesh "NoCollision")
        (Utilities|FlowControl|Delay (Variables|Default|GetrespawnTime))
        (Collision|SetCollisionEnabled _staticmesh "QueryAndPhysics")
        (bind _transparency_2 (Timeline|ReverseTransparancy ReverseFromEnd)
          (:Update
            (Rendering|Material|SetScalarParameterValue _cloudpaint "Transparency" _transparency_2 :!class /Script/Engine.MaterialInstanceDynamic))
          (:Finished
            (Variables|Default|SetalreadyHit false)))))))

(event EventBeginPlay)

(event Collision|EventActorBeginOverlap
  (params (OtherActor :type Actor%20Object%20Reference)))

(event EventTick
  (params (DeltaSeconds :type Float%20%28single-precision%29)))

(fn ConstructionScript
  (bind _returnvalue (Rendering|Material|CreateDynamicMaterialInstance (Variables|Default|GetStaticMesh) 0 0 "None" :!class /Script/Engine.PrimitiveComponent))
  (Variables|Default|SetCloudPaint _returnvalue))