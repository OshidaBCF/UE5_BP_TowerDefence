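; BP_Tower is an automatic turret that shoots projectiles at the nearest actor tagged "Enemy".
; A looping timer searches all tagged actors for the closest one, then picks the left or right Niagara component as muzzle from the yaw toward it.
; If that enemy is within Range of the muzzle, it spawns a BP_Projectile there and launches its Arrow toward the target with an impulse scaled by Force.
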(event Custom|Check
  (bind _tower (Variables|Default|GetTower))
  (bind _outactors (Actor|GetAllActorswithTag "Enemy"))
  (switch int (Utilities|Array|Length _outactors)
    (:Default
      (for (_array_element _array_index) _outactors
        (if (== _array_index 0)
          (Variables|Default|SetclosestEnemy _array_element :!label _label)
          (elif (< (Transformation|GetDistanceTo _array_element) (Transformation|GetDistanceTo (Variables|Default|GetclosestEnemy)))
            (goto _label))))
      (if (< (Math|Vector|VectorLength (- (Transformation|GetActorLocation (Variables|Default|GetclosestEnemy)) (Transformation|GetWorldLocation (select (Math|Float|InRange(Float) (.Yaw (Math|Rotator|BreakRotator (Math|Rotator|CombineRotators (Transformation|GetWorldRotation _tower) (Math|Rotator|FindLookatRotation (Transformation|GetWorldLocation _tower) (Transformation|GetActorLocation (Variables|Default|GetclosestEnemy)))))) -9e+01 9e+01) (Variables|Default|GetrightNiagara) (Variables|Default|GetleftNiagara))))) (Variables|Default|Getrange))
        (bind _returnvalue (Game|SpawnActorfromClass "/Game/MyBPs/BP_Projectile.BP_Projectile_C" (Math|Transform|MakeTransform (Transformation|GetWorldLocation (select (Math|Float|InRange(Float) (.Yaw (Math|Rotator|BreakRotator (Math|Rotator|CombineRotators (Transformation|GetWorldRotation _tower) (Math|Rotator|FindLookatRotation (Transformation|GetWorldLocation _tower) (Transformation|GetActorLocation (Variables|Default|GetclosestEnemy)))))) -9e+01 9e+01) (Variables|Default|GetrightNiagara) (Variables|Default|GetleftNiagara))) (Math|Rotator|FindLookatRotation (Transformation|GetWorldLocation (select (Math|Float|InRange(Float) (.Yaw (Math|Rotator|BreakRotator (Math|Rotator|CombineRotators (Transformation|GetWorldRotation _tower) (Math|Rotator|FindLookatRotation (Transformation|GetWorldLocation _tower) (Transformation|GetActorLocation (Variables|Default|GetclosestEnemy)))))) -9e+01 9e+01) (Variables|Default|GetrightNiagara) (Variables|Default|GetleftNiagara))) (Transformation|GetActorLocation (Variables|Default|GetclosestEnemy)))) "AlwaysSpawn" "MultiplyWithRoot" 0 0))
        (Physics|AddImpulse (Variables|/Game/MyBPs/BP_Projectile.BP_Projectile_C|GetArrow _returnvalue) (* (Math|Vector|Normalize (- (Transformation|GetActorLocation (Variables|Default|GetclosestEnemy)) (Transformation|GetWorldLocation (select (Math|Float|InRange(Float) (.Yaw (Math|Rotator|BreakRotator (Math|Rotator|CombineRotators (Transformation|GetWorldRotation _tower) (Math|Rotator|FindLookatRotation (Transformation|GetWorldLocation _tower) (Transformation|GetActorLocation (Variables|Default|GetclosestEnemy)))))) -9e+01 9e+01) (Variables|Default|GetrightNiagara) (Variables|Default|GetleftNiagara))))) (Variables|Default|Getforce)) "None" true)))))

(event EventBeginPlay
  (Utilities|Time|SetTimerbyEvent (delegate Custom|Check) 2.0 true))

(event Collision|EventActorBeginOverlap
  (params (OtherActor :type Actor%20Object%20Reference)))

(event EventTick
  (params (DeltaSeconds :type Float%20%28single-precision%29)))

(fn ConstructionScript)