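; BP_greenball is a ball Blueprint that tries to drive its Sphere component along its forward vector.
; Each Tick scales the forward vector by Speed and delta time, then multiplies it by the world location instead of adding it to set the new position.
; A separate missile graph holds a custom event with the same math plus a multiply by world rotation; nothing in the file calls it.
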(event EventTick
  (params (DeltaSeconds :type Float%20%28single-precision%29))
  (Transformation|SetWorldLocation (Variables|Default|GetSphere) (* (* (* DeltaSeconds (Variables|Default|GetSpeed)) (Math|Vector|GetForwardVector (Variables|Default|GetSphere))) (Transformation|GetWorldLocation (Variables|Default|GetSphere))) false false))

(event Custom|CustomEvent
  (params (DeltaSeconds :type Float%20%28single-precision%29))
  (Transformation|SetWorldLocation (Variables|Default|GetSphere) (* (* (* (* DeltaSeconds (Variables|Default|GetSpeed)) (Math|Vector|GetForwardVector (Variables|Default|GetSphere))) (Transformation|GetWorldLocation (Variables|Default|GetSphere))) (Transformation|GetWorldRotation (Variables|Default|GetSphere))) false false))

(fn ConstructionScript)